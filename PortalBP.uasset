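; PortalBP is a paired teleporter that moves the FirstPersonCharacter to the linked portal's Exit point when the character hits it.
; On each hit it scans all PortalBP actors for one with the same PortalIndex and the opposite IsEnterance flag, so travel works both ways.
; The construction script positions the portal body and Exit from per-instance variables and tints the body through a dynamic material instance.
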(event Collision|EventHit
  (params (MyComp :type Primitive%20Component%20Object%20Reference) (Other :type Actor%20Object%20Reference) (OtherComp :type Primitive%20Component%20Object%20Reference) (bSelfMoved :type Boolean) (HitLocation :type Vector :default "0, 0, 0") (HitNormal :type Vector :default "0, 0, 0") (NormalImpulse :type Vector :default "0, 0, 0") (Hit :type Hit%20Result%20Structure%20%28by%20ref%29))
  (bind _asfirst_person_character (Utilities|Casting|CastToFirstPersonCharacter Other))
  (if (Variables|Default|GetIsEnterance)
    (bind _outactors (Actor|GetAllActorsOfClass "PortalBP_C"))
    (bind _array_element (Utilities|Array|ForEachLoopwithBreak _outactors :!label _label)
      (:LoopBody
        (if (and (== (Variables|PortalBP_C|GetPortalIndex _array_element) (Variables|Default|GetPortalIndex)) (not (Variables|PortalBP_C|GetIsEnterance _array_element)))
          (goto _label Break)))
      (:Completed
        (Transformation|SetActorLocation _asfirst_person_character (Transformation|GetWorldLocation (Variables|PortalBP_C|GetExit _array_element)) false false)))
    (else
      (bind _outactors_2 (Actor|GetAllActorsOfClass "PortalBP_C"))
      (bind _array_element_2 (Utilities|Array|ForEachLoopwithBreak _outactors_2 :!label _label_2)
        (:LoopBody
          (if (and (== (Variables|PortalBP_C|GetPortalIndex _array_element_2) (Variables|Default|GetPortalIndex)) (and (not (Variables|Default|GetIsEnterance)) (Variables|PortalBP_C|GetIsEnterance _array_element_2)))
            (goto _label_2 Break)))
        (:Completed
          (Transformation|SetActorLocation _asfirst_person_character (Transformation|GetWorldLocation (Variables|PortalBP_C|GetExit _array_element_2)) false false))))))

(fn ConstructionScript
  (bind _portalbody (Variables|Default|GetPortalBody))
  ;[1 1 1] Setting portal locations including exit
  (Transformation|SetRelativeTransform (Variables|Default|GetPortalBody) (Variables|Default|GetPortalTransform) false false)
  (Transformation|SetRelativeLocation (Variables|Default|GetExit) (Variables|Default|GetExitLocation) false false)
  ;[1 1 1] Set colour
  (bind _returnvalue (Rendering|Material|CreateDynamicMaterialInstance _portalbody 0 "/Game/Blueprints/Portal/PortalMaterial_Inst.PortalMaterial_Inst" "None" :!class /Script/Engine.PrimitiveComponent))
  (Rendering|Material|SetVectorParameterValue _returnvalue "Colour" (Variables|Default|GetColour) :!class /Script/Engine.MaterialInstanceDynamic)
  (Rendering|Material|SetMaterial _portalbody 0 _returnvalue))